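; ConstructionManager_BP manages building construction in the strategy game, swapping placeholder proxies for finished buildings.
; QueueConstruction spawns a proxy with the display mesh from the construction struct, binds its completion event, and stores proxy and struct in parallel arrays.
; On completion, FinishConstruction finds the struct by the proxy's index, removes both entries, spawns the building at the stored transform and destroys the proxy.
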(event Custom|BindConstruction
  (params (Proxy :type Construction%20Proxy%20BP%20Object%20Reference))
  (EventDispatchers|BindEventtoConstructionComplete Proxy (EventDispatchers|CreateEvent :!event Custom|ConstructionComplete)))

(event Custom|ConstructionComplete
  (params (Proxy :type Construction%20Proxy%20BP%20Object%20Reference))
  (CallFunction|FinishConstruction Proxy))

(fn ConstructionScript)

(fn QueueConstruction
  (params (ConstructionDS :type Construction%20DS%20Structure))
  (bind (_buildingclass _proxyclass _transform _displaymesh) (Utilities|Struct|BreakConstruction_DS ConstructionDS))
  (bind _returnvalue (Game|SpawnActorfromClass _proxyclass _transform "AlwaysSpawn" 0 _displaymesh 0))
  (CallFunction|BindConstruction _returnvalue)
  (Utilities|Array|Add (Variables|Default|GetProxies) _returnvalue)
  (Utilities|Array|Add (Variables|Default|GetQueue) ConstructionDS))

(fn FinishConstruction
  (params (Proxy :type Construction%20Proxy%20BP%20Object%20Reference))
  (bind _proxies (Variables|Default|GetProxies))
  (bind _queue (Variables|Default|GetQueue))
  (bind _output_get (LocalVariables|SetIndex (Utilities|Array|FindItem _proxies Proxy)))
  (LocalVariables|SetConfiguration (Utilities|Array|Get(acopy) _queue _output_get))
  (Utilities|Array|RemoveIndex _queue (LocalVariables|GetIndex))
  (Utilities|Array|RemoveIndex _proxies (LocalVariables|GetIndex))
  (Game|SpawnActorfromClass (.BuildingClass (Utilities|Struct|BreakConstruction_DS (LocalVariables|GetConfiguration))) (.Transform (Utilities|Struct|BreakConstruction_DS (LocalVariables|GetConfiguration))) "Undefined" 0 0 0)
  (Actor|DestroyActor Proxy))