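; ConstructionProxy_BP is a building construction proxy for the strategy game that shows a display mesh and tracks construction time.
; The construction script applies DisplayMesh and the test building material to its static mesh.
; SetBuildingConstructionTime converts creation hours to minutes, while BuildingWork advances a clock via SetClockWork to derive the time spent.
; Tick calls CallConstructionComplete on itself every frame.
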(event EventTick
  (params (DeltaSeconds :type Float%20%28single-precision%29))
  (Default|CallConstructionComplete self))

(fn ConstructionScript
  (bind _staticmesh (Variables|Default|GetStaticMesh))
  (Components|StaticMesh|SetStaticMesh _staticmesh (Variables|Default|GetDisplayMesh))
  (Rendering|Material|SetMaterial _staticmesh 0 "/Game/Strategy_Game/Materials/TestBuilding_Norm_Material.TestBuilding_Norm_Material"))

(fn SetBuildingConstructionTime
  (params (CreationHours :type Float%20%28single-precision%29))
  (Variables|Default|SetConstructionTime (* CreationHours 6e+01))
  (return))

(fn BuildingWork
  (bind _output_get (Variables|Default|SetClockWork (.ClockWorkOut (CallFunction|SetClockWork (Variables|Default|GetDeltaSec) (Variables|Default|GetTimeUnit) (Variables|Default|GetClockWork)))))
  (Variables|Default|SetConstructionTimeSpent (* _output_get 6e+01))
  (return))