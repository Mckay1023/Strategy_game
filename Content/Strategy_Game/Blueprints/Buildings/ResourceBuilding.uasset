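; Resource building Blueprint for a strategy game that periodically adds resources to the player.
; On BeginPlay it starts a looping function-name timer that calls IncreaseResources.
; IncreaseResources adds IncreaseAmount to the Resources total on player 0's CameraPawnController and prints a message.
; A ResourceTimerClear event stops the timer by clearing its stored handle.
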(event Custom|ResourceTimer
  (bind _returnvalue (Utilities|Time|SetTimerbyFunctionName 0 "IncreaseResources" 3e+01 true)))

(event Custom|ResourceTimerClear
  (Utilities|Time|ClearandInvalidateTimerbyHandle (stale Custom|ResourceTimer _returnvalue)))

(event EventBeginPlay
  (CallFunction|ResourceTimer))

(fn ConstructionScript
  (|CallParentFunction))

(fn IncreaseResources
  (bind _ascamera_pawn_controller (Utilities|Casting|CastToCameraPawnController (Game|GetPlayerController 0)))
  (Variables|/Game/Strategy_Game/Blueprints/CameraPawnController.CameraPawnController_C|SetResources _ascamera_pawn_controller (+ (Variables|/Game/Strategy_Game/Blueprints/CameraPawnController.CameraPawnController_C|GetResources _ascamera_pawn_controller) (LocalVariables|GetIncreaseAmount)))
  (Development|PrintString (LocalVariables|GetResourceIncrease))
  (return))