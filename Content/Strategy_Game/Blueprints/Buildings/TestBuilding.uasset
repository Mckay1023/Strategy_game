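; Placement preview actor for the strategy game, showing the selected building's mesh at a grid-snapped cursor position.
; CreateBuilding briefly spawns the building class to read its display mesh and construction proxy class, restarts the preview, then destroys that actor.
; Spawn and kill toggle the camera controller's BuildingActivated flag and a Tick gate that moves the preview.
; GetConstructionDS packages the classes, mesh and transform as construction data.
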(event Custom|OnBuildingSpawn
  (params (DisplayMesh :type Static%20Mesh%20Object%20Reference) (GameBuildingClass :type M%20Game%20Buildings%20Class%20Reference) (ConstructionProxyClass :type Construction%20Proxy%20BP%20Class%20Reference))
  ;[1 1 1] Spawn of building
  (if (not (Variables|Default|GetIsActive))
    (Variables|Default|SetGameBuildingClass GameBuildingClass)
    (Variables|Default|SetConstructionProxyClass ConstructionProxyClass)
    (Variables|Default|SetDisplayMesh DisplayMesh)
    (Variables|Default|SetIsActive true)
    (Variables|/Game/Strategy_Game/Blueprints/CameraPawnController.CameraPawnController_C|SetBuildingActivated (Variables|Default|GetCameraControllerRef) true)
    (Components|StaticMesh|SetStaticMesh (Variables|Default|GetTestBuildingMesh) (Variables|Default|GetDisplayMesh))
    (CallFunction|OpenTickGate)))

(event Custom|KillTestBuilding
  ;[1 1 1] Kill Test Building
  (Variables|Default|SetGameBuildingClass 0)
  (Variables|Default|SetConstructionProxyClass 0)
  (CallFunction|CloseTickGate)
  (Variables|Default|SetDisplayMesh 0)
  (Variables|Default|SetIsActive false)
  (Variables|/Game/Strategy_Game/Blueprints/CameraPawnController.CameraPawnController_C|SetBuildingActivated (Variables|Default|GetCameraControllerRef) false)
  (Components|StaticMesh|SetStaticMesh (Variables|Default|GetTestBuildingMesh) (Variables|Default|GetDisplayMesh)))

(event Custom|OpenTickGate
  (Utilities|FlowControl|Gate true) ; enters at Open
)

(event Custom|CloseTickGate
  (Utilities|FlowControl|Gate true) ; enters at Close
)

(event EventCreateBuilding
  (params (GameBuilding :type M%20Game%20Buildings%20Class%20Reference))
  ;[1 1 1] Create Building
  (bind _returnvalue (Game|SpawnActorfromClass GameBuilding (Math|Transform|MakeTransform "0, 0, 0") "AlwaysSpawn" 0 (Variables|Default|GetCameraControllerRef) 0))
  (Utilities|FlowControl|Sequence
    (:then_0
      (bind _asm_game_buildings (Utilities|Casting|CastToM_GameBuildingsClass GameBuilding))
      (CallFunction|KillTestBuilding)
      (CallFunction|OnBuildingSpawn (Variables|/Game/Strategy_Game/Blueprints/Buildings/M_GameBuildings.M_GameBuildings_C|GetDisplayMesh _returnvalue) _asm_game_buildings (Variables|/Game/Strategy_Game/Blueprints/Buildings/M_GameBuildings.M_GameBuildings_C|GetConstructionProxyClass _returnvalue)))
    (:then_1
      (Actor|DestroyActor _returnvalue))))

(event EventTick
  (params (DeltaSeconds :type Float%20%28single-precision%29))
  (Utilities|FlowControl|Gate true
    (:Exit
      (Transformation|SetActorLocation self (CallFunction|SetGridSnap) false false))))

(fn ConstructionScript)

(fn SetGridSnap
  (bind _cursorposition (Variables|Default|GetCursorPosition))
  (bind _gridsize (Variables|Default|GetGridSize))
  (return (Math|Vector|MakeVector (CallFunction|GridSnap (.x _cursorposition) _gridsize) (CallFunction|GridSnap (.y _cursorposition) _gridsize) (CallFunction|GridSnap (.z _cursorposition) _gridsize))))

(fn SetCursorPosition
  (params (CursorLocation :type Vector))
  (Variables|Default|SetCursorPosition CursorLocation)
  (return))

(fn GetConstructionDS
  (return (Utilities|Struct|MakeConstruction_DS (Variables|Default|GetGameBuildingClass) (Variables|Default|GetConstructionProxyClass) (Math|Transform|MakeTransform (Transformation|GetActorLocation) (Transformation|GetActorRotation)) (Variables|Default|GetDisplayMesh) 1.0)))

(fn SetClock
  (params (ClockTime :type Array%20of%20Integers))
  (return false))