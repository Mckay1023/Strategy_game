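; Player controller for a strategy game that drives the camera pawn, building placement and a resource counter.
; Axis and action inputs pan, yaw and zoom the pawn's spring-arm camera.
; BeginPlay spawns ConstructionManager and TestBuilding, creates the HUD and starts a looping timer that adds resources.
; While placement is active, Tick moves TestBuilding to the cursor using a zoom-adjusted distance; left click queues construction and removes the preview.
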(event Custom|TimeBonus
  ;[1 1 1] TimeBonus
  (bind _returnvalue (Utilities|Time|SetTimerbyFunctionName self "AddTimeResources" 1e+01 true)))

(event Custom|CustomEvent_0
  ;[1 1 1] TimeBonus
  (Utilities|Time|ClearandInvalidateTimerbyHandle (stale Custom|TimeBonus _returnvalue)))

(event EventBeginPlay
  (bind _returnvalue (Math|Transform|MakeTransform "0, 0, 0"))
  ;[1 1 1] Begin Play
  (Utilities|FlowControl|Sequence
    (:then_0
      (Utilities|ReferenceCasts)
      (CallFunction|TimeBonus))
    (:then_1
      (bind _returnvalue_2 (Game|SpawnActorfromClass "/Game/Strategy_Game/Blueprints/Construction/ConstructionManager_BP.ConstructionManager_BP_C" _returnvalue "AlwaysSpawn" 0 0))
      (Variables|References|SetConstructionManagerRef _returnvalue_2))
    (:then_2
      (bind _returnvalue_3 (Game|SpawnActorfromClass "/Game/Strategy_Game/Blueprints/Buildings/TestBuilding.TestBuilding_C" _returnvalue "AlwaysSpawn" 0 self 0))
      (Variables|References|SetTestBuildingRef _returnvalue_3))
    (:then_3
      (Input|SetInputModeGameandUI self 0 "LockAlways" false)
      (Utilities|CreateHUDs)
      (UserInterface|Viewport|AddtoViewport (Variables|References|GetGameHudRef) 0))))

(event EventTick
  (params (DeltaSeconds :type Float%20%28single-precision%29))
  ;[1 1 1] Event Tick
  (if (Variables|Default|GetBuildingActivated)
    (|SetCursorLocation)))

(event Input|ActionEvents|InputActionZoomIn
  (params (Key :type Key%20Structure))
  (bind _mycamerapawnref (Variables|References|GetMyCameraPawnRef))
  (bind _mycameraspringarm (Variables|/Script/Strategy_game.MyCameraPawn|GetMyCameraSpringArm _mycamerapawnref))
  ;[1 1 1] Zoom In and Out
  (:Pressed
    (Variables|/Script/Engine.SpringArmComponent|SetTargetArmLength _mycameraspringarm (Math|Float|Clamp(Float) (- (Variables|/Script/Engine.SpringArmComponent|GetTargetArmLength _mycameraspringarm) (Variables|Default|GetZoomSpeed)) 1e+03 (Variables|Default|GetMaxArmDistance)))))

(event Input|ActionEvents|InputActionZoomOut
  (params (Key :type Key%20Structure))
  (bind _mycamerapawnref (Variables|References|GetMyCameraPawnRef))
  (bind _mycameraspringarm (Variables|/Script/Strategy_game.MyCameraPawn|GetMyCameraSpringArm _mycamerapawnref))
  ;[1 1 1] Zoom In and Out
  (:Pressed
    (Variables|/Script/Engine.SpringArmComponent|SetTargetArmLength _mycameraspringarm (Math|Float|Clamp(Float) (+ (Variables|Default|GetZoomSpeed) (Variables|/Script/Engine.SpringArmComponent|GetTargetArmLength _mycameraspringarm)) 1e+02 (Variables|Default|GetMaxArmDistance)))))

(event Input|ActionEvents|InputActionDeselect
  (params (Key :type Key%20Structure))
  ;[1 1 1] Deselect/Drop Building
  (:Pressed
    (if (Variables|Default|GetBuildingActivated)
      (Default|KillTestBuilding (Variables|References|GetTestBuildingRef))
      (Variables|Default|SetBuildingActivated false))))

(event Input|AxisEvents|InputAxisMoveForward
  (params (AxisValue :type Float%20%28single-precision%29))
  (bind _mycamerapawnref (Variables|References|GetMyCameraPawnRef))
  (bind _returnvalue (Transformation|GetActorTransform _mycamerapawnref))
  (bind (_location _rotation _scale) (Math|Transform|BreakTransform _returnvalue))
  ;[1 1 1] Move Forward and Backwards
  (Transformation|SetActorTransform (Variables|References|GetMyCameraPawnRef) (Math|Transform|MakeTransform (+ (Math|Transform|TransformDirection _returnvalue (Math|Vector|MakeVector (* AxisValue (Variables|Default|GetMovementSpeed)) 0.0 0.0)) _location) _rotation _scale)))

(event Input|AxisEvents|InputAxisMoveRight
  (params (AxisValue :type Float%20%28single-precision%29))
  (bind _mycamerapawnref (Variables|References|GetMyCameraPawnRef))
  (bind _returnvalue (Transformation|GetActorTransform _mycamerapawnref))
  (bind (_location _rotation _scale) (Math|Transform|BreakTransform _returnvalue))
  ;[1 1 1] Move Right and Left
  (Transformation|SetActorTransform (Variables|References|GetMyCameraPawnRef) (Math|Transform|MakeTransform (+ (Math|Transform|TransformDirection _returnvalue (Math|Vector|MakeVector 0.0 (* AxisValue (Variables|Default|GetMovementSpeed)) 0.0)) _location) _rotation _scale)))

(event Input|AxisEvents|InputAxisCameraPitch
  (params (AxisValue :type Float%20%28single-precision%29))
  ;[1 1 1] Rotate Camera Pitch-- disconnected
)

(event Input|AxisEvents|InputAxisCameraYaw
  (params (AxisValue :type Float%20%28single-precision%29))
  (bind _mycamerapawnref (Variables|References|GetMyCameraPawnRef))
  (bind _returnvalue (Transformation|GetActorRotation _mycamerapawnref))
  (bind (_roll _pitch _yaw) (Math|Rotator|BreakRotator _returnvalue))
  ;[1 1 1] Rotate Camera Yaw
  (Transformation|SetActorRotation (Variables|References|GetMyCameraPawnRef) (Math|Rotator|MakeRotator _roll _pitch (+ AxisValue _yaw))))

(event Input|MouseEvents|LeftMouseButton
  (params (Key :type Key%20Structure))
  ;[1 1 1] Deselect/Drop Building
  (:Pressed
    (if (Variables|Default|GetBuildingActivated)
      (bind _constructionds (Default|GetConstructionDS (Variables|References|GetTestBuildingRef)))
      (Default|QueueConstruction (Variables|References|GetConstructionManagerRef) _constructionds)
      (Default|KillTestBuilding (Variables|References|GetTestBuildingRef)))))

(fn ConstructionScript)

(fn SetDistancePlacement
  (return (+ (Variables|Default|GetDistancePlacement) (Variables|/Script/Engine.SpringArmComponent|GetTargetArmLength (Variables|/Script/Strategy_game.MyCameraPawn|GetMyCameraSpringArm (Variables|References|GetMyCameraPawnRef))))))

(fn AddTimeResources
  (Variables|Default|SetResources (+ (Variables|Default|GetResources) 20))
  (Development|PrintString (Utilities|String|ToString(Integer) (Variables|Default|GetResources))))

(fn AddtoPlayerResources
  (params (Minutes :type Integer))
  (if (== (Math|Float|Truncate (.Remainder (Math|Float|Division(WholeandRemainder) (Math|Conversions|ToFloat(Integer) Minutes) 1e+01))) 0)
    (Variables|Default|SetResources (+ (Variables|Default|GetResources) 25))))

(fn SetClock
  (params (ClockTime :type Array%20of%20Integers))
  (return false))